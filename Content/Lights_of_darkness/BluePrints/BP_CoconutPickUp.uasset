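; BP_CoconutPickUp is a coconut food pickup that restores the third-person character's hunger when the player interacts nearby.
; A box overlap shows a prompt widget, caches the character and opens a Gate, which closes again when the character leaves.
; While the gate is open, the interact input adds a clamped amount to Hunger, refreshes it, plays a pickup sound and destroys the actor.
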(event `self.ReceiveBeginPlay`
  (`self.EnableInput` (`GameplayStatics.GetPlayerController` 0)))

(event `EnhancedInput|/Game/ThirdPerson/Input/Actions/IA_Interact`
  (params (ActionValue :type Boolean) (ElapsedSeconds :type "Float (double-precision)") (TriggeredSeconds :type "Float (double-precision)") (InputAction :type "InputAction Object Reference" :default "/Game/ThirdPerson/Input/Actions/IA_Interact.IA_Interact"))
  (:`Triggered`
    (`/Engine/EditorBlueprintResources/StandardMacros.Gate` true :!label _label
      (:`Exit`
        (`/Engine/EditorBlueprintResources/StandardMacros.IsValid` (stale `self.Box.OnComponentBeginOverlap` _asbp_third_person_character)
          (:`Is Valid`
            (set `/Game/ThirdPerson/Blueprints/BP_ThirdPersonCharacter.Hunger` (`KismetMathLibrary.FClamp` (+ (`/Game/ThirdPerson/Blueprints/BP_ThirdPersonCharacter.Hunger` (stale `self.Box.OnComponentBeginOverlap` _asbp_third_person_character)) 20.0) 0.0 100.0) (stale `self.Box.OnComponentBeginOverlap` _asbp_third_person_character))
            (`/Game/ThirdPerson/Blueprints/BP_ThirdPersonCharacter.UpdateHunger` (stale `self.Box.OnComponentBeginOverlap` _asbp_third_person_character))
            (`GameplayStatics.PlaySoundAtLocation` "/Game/Lights_of_darkness/Sounds/PickupCoconut/411177__silverillusionist__pick-up-item-1.411177__silverillusionist__pick-up-item-1" (`self.K2_GetActorLocation`) (struct) 1.0 1.0 0.0 null null null null)
            (`self.K2_DestroyActor`)))))))

(event `self.Box.OnComponentBeginOverlap`
  (params (OverlappedComponent :type "PrimitiveComponent Object Reference") (OtherActor :type "Actor Object Reference") (OtherComp :type "PrimitiveComponent Object Reference") (OtherBodyIndex :type Integer) (bFromSweep :type Boolean) (SweepResult :type "HitResult Structure (by ref)"))
  (`SceneComponent.SetVisibility` (`self.Widget`) true false)
  (bind _asbp_third_person_character (cast `/Game/ThirdPerson/Blueprints/BP_ThirdPersonCharacter` OtherActor))
  (goto _label :!via `Open`))

(event `self.Box.OnComponentEndOverlap`
  (params (OverlappedComponent :type "PrimitiveComponent Object Reference") (OtherActor :type "Actor Object Reference") (OtherComp :type "PrimitiveComponent Object Reference") (OtherBodyIndex :type Integer))
  (`SceneComponent.SetVisibility` (`self.Widget`) false false)
  (cast `/Game/ThirdPerson/Blueprints/BP_ThirdPersonCharacter` OtherActor)
  (goto _label :!via `Close`))

(fn `UserConstructionScript`)