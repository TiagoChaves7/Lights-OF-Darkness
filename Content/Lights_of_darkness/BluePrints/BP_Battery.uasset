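; BP_Battery is a battery pickup that the third-person character collects with the Interact input.
; It enables input for player controller 0 on BeginPlay.
; Box overlap shows or hides a widget for any actor, while only the character opens or closes the gate that lets Interact through.
; An accepted Interact calls BatteryPickup on the cached character, plays a pickup sound at its location and destroys the battery.
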(event `self.ReceiveBeginPlay`
  (`self.EnableInput` (`GameplayStatics.GetPlayerController` 0)))

(event `EnhancedInput|/Game/ThirdPerson/Input/Actions/Interact`
  (params (ActionValue :type Boolean) (ElapsedSeconds :type "Float (double-precision)") (TriggeredSeconds :type "Float (double-precision)") (InputAction :type "InputAction Object Reference" :default "/Game/ThirdPerson/Input/Actions/Interact.Interact"))
  (:`Triggered`
    (`/Engine/EditorBlueprintResources/StandardMacros.Gate` true :!label _label
      (:`Exit`
        (`/Game/ThirdPerson/Blueprints/BP_ThirdPersonCharacter.Battery Pickup` (stale `self.Box.OnComponentBeginOverlap` _asbp_third_person_character))
        (`GameplayStatics.PlaySoundAtLocation` "/Game/Lights_of_darkness/Sounds/PickUpFlower/240784__f4ngy__picking-flower.240784__f4ngy__picking-flower" (`self.K2_GetActorLocation`) (struct) 1.0 1.0 0.0 null null null null)
        (`self.K2_DestroyActor`)))))

(event `self.Box.OnComponentBeginOverlap`
  (params (OverlappedComponent :type "PrimitiveComponent Object Reference") (OtherActor :type "Actor Object Reference") (OtherComp :type "PrimitiveComponent Object Reference") (OtherBodyIndex :type Integer) (bFromSweep :type Boolean) (SweepResult :type "HitResult Structure (by ref)"))
  (`SceneComponent.SetVisibility` (`self.Widget`) true false)
  (bind _asbp_third_person_character (cast `/Game/ThirdPerson/Blueprints/BP_ThirdPersonCharacter` OtherActor))
  (goto _label :!via `Open`))

(event `self.Box.OnComponentEndOverlap`
  (params (OverlappedComponent :type "PrimitiveComponent Object Reference") (OtherActor :type "Actor Object Reference") (OtherComp :type "PrimitiveComponent Object Reference") (OtherBodyIndex :type Integer))
  (`SceneComponent.SetVisibility` (`self.Widget`) false false)
  (cast `/Game/ThirdPerson/Blueprints/BP_ThirdPersonCharacter` OtherActor)
  (goto _label :!via `Close`))

(fn `UserConstructionScript`)